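; TensionBeam is a short-lived weapon actor that destroys itself 0.4 seconds after spawning.
; Its capsule overlap runs a cast chain, destroying Baddie, BaddieBob and BaddieWave with an explosion and sound, and calling AddToScore on the player's ShootingCharacter.
; Tension beam and shield pickups are destroyed the same way without scoring.
; BaddieBoss instead loses one Health with a shock effect, and the beam persists through hits.
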(event `/Game/Blueprints/ShotPlain.ReceiveBeginPlay`
  (`KismetSystemLibrary.Delay` 0.4)
  (`self.K2_DestroyActor`))

(event `self.Capsule.OnComponentBeginOverlap`
  (params (OtherActor :type "Actor Object Reference") (OtherComp :type "PrimitiveComponent Object Reference") (OtherBodyIndex :type Integer) (bFromSweep :type Boolean) (SweepResult :type "HitResult Structure (by ref)"))
  (bind _asbaddie (cast `/Game/Blueprints/Baddie` OtherActor)
    (:`then`
      (`GameplayStatics.SpawnEmitterAtLocation` "/Game/PARTICLES/A_Boom.A_Boom" (`self.K2_GetActorLocation` _asbaddie))
      (`self.K2_DestroyActor` _asbaddie)
      (bind _asshooting_character (cast `/Game/Blueprints/ShootingCharacter` (`GameplayStatics.GetPlayerCharacter` 0) :!label _label))
      (`/Game/Blueprints/ShootingCharacter.AddToScore` _asshooting_character)
      (`GameplayStatics.PlaySoundAtLocation` "/Game/noise/hit_Cue.hit_Cue" (`self.K2_GetActorLocation`) :!label _label_2))
    (:`CastFailed`
      (bind _asbaddie_bob (cast `/Game/Blueprints/BaddieBob` OtherActor)
        (:`then`
          (`GameplayStatics.SpawnEmitterAtLocation` "/Game/PARTICLES/A_Boom.A_Boom" (`self.K2_GetActorLocation` _asbaddie_bob))
          (`self.K2_DestroyActor` _asbaddie_bob)
          (goto _label))
        (:`CastFailed`
          (bind _asbaddie_wave (cast `/Game/Blueprints/BaddieWave` OtherActor)
            (:`then`
              (`GameplayStatics.SpawnEmitterAtLocation` "/Game/PARTICLES/A_Boom.A_Boom" (`self.K2_GetActorLocation` _asbaddie_wave))
              (`self.K2_DestroyActor` _asbaddie_wave)
              (goto _label))
            (:`CastFailed`
              (bind _aspickup_tension_beam (cast `/Game/Blueprints/Pickup_tensionBeam` OtherActor)
                (:`then`
                  (`GameplayStatics.SpawnEmitterAtLocation` "/Game/PARTICLES/A_Boom.A_Boom" (`self.K2_GetActorLocation` _aspickup_tension_beam))
                  (`self.K2_DestroyActor` _aspickup_tension_beam)
                  (goto _label_2))
                (:`CastFailed`
                  (bind _aspickup_shield (cast `/Game/Blueprints/Pickup_shield` OtherActor)
                    (:`then`
                      (`GameplayStatics.SpawnEmitterAtLocation` "/Game/PARTICLES/A_Boom.A_Boom" (`self.K2_GetActorLocation` _aspickup_shield))
                      (`self.K2_DestroyActor` _aspickup_shield)
                      (goto _label_2))
                    (:`CastFailed`
                      (bind _asbaddie_boss (cast `/Game/Blueprints/BaddieBoss` OtherActor))
                      (`GameplayStatics.SpawnEmitterAtLocation` "/Game/PARTICLES/A_Shock.A_Shock" (`SceneComponent.K2_GetComponentLocation` (`self.Capsule`)) (struct))
                      (set `/Game/Blueprints/BaddieBoss.Health` (- (`/Game/Blueprints/BaddieBoss.Health` _asbaddie_boss) 1) _asbaddie_boss))))))))))))

(fn `UserConstructionScript`)