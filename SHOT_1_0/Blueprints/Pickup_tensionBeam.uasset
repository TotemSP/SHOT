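; Tension beam pickup that grants the beam to a ShootingCharacter on touch and expires if left uncollected.
; A sphere overlap casts to ShootingCharacter, calls TBeamGet, spawns a pulse particle effect and destroys the actor.
; BeginPlay starts a timed delay that destroys the pickup.
; The construction script tints the beam and ring components through dynamic instances of a shared item material.
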(event `self.ReceiveBeginPlay`
  (`KismetSystemLibrary.Delay` 20.0)
  (`self.K2_DestroyActor`))

(event `self.Sphere.OnComponentBeginOverlap`
  (params (OtherActor :type "Actor Object Reference") (OtherComp :type "PrimitiveComponent Object Reference") (OtherBodyIndex :type Integer) (bFromSweep :type Boolean) (SweepResult :type "HitResult Structure (by ref)"))
  (bind _asshooting_character (cast `/Game/Blueprints/ShootingCharacter` OtherActor))
  (`/Game/Blueprints/ShootingCharacter.TBeamGet` _asshooting_character)
  (`GameplayStatics.SpawnEmitterAtLocation` "/Game/PARTICLES/A_Pulse.A_Pulse" (`self.K2_GetActorLocation`))
  (`self.K2_DestroyActor`))

(fn `UserConstructionScript`
  (bind _returnvalue (`PrimitiveComponent.CreateDynamicMaterialInstance` (`self.TBeam`) 0 "/Game/MAT/Item_Mat.Item_Mat"))
  (`MaterialInstanceDynamic.SetVectorParameterValue` _returnvalue "Colour" (struct :`R` 1.0 :`A` 1.0))
  (bind _returnvalue_2 (`PrimitiveComponent.CreateDynamicMaterialInstance` (`self.Pickup_ring`) 0 "/Game/MAT/Item_Mat.Item_Mat"))
  (`MaterialInstanceDynamic.SetVectorParameterValue` _returnvalue_2 "Colour" (struct :`R` 1.0 :`G` 1.0 :`A` 1.0)))