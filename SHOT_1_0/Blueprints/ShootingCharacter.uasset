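; Player ship for a side-scrolling shooter, with auto-scroll movement that stops when a timed boss flag sets.
; Pickup events restore the shield or grant the Tension Beam, scoring points for duplicates; Tick fades shield opacity through a dynamic material.
; Fire repeats shots under an on-screen cap, while the beam runs delay-timed charge, firing and heat-vent phases.
; Death spawns a wreck and notifies the game mode, unless debug mode is on.
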(event `Shield GET`
  ;[1 1 1] Shield systems on GET event
  (if (`self.IsShieldDown`)
    (set `self.IsShieldDown` false)
    (`GameplayStatics.PlaySound2D` "/Game/noise/Shieldget_Cue.Shieldget_Cue")
    (set `self.ShieldGot` true)
    (set `self.Opacity` 1.0)
    (`ActorComponent.SetActive` (`self.Charging`) true false)
    (elif (not (`self.DebugMode`))
      (set `self.Score` (+ (`self.Score`) 10))
      (`GameplayStatics.PlaySound2D` "/Game/noise/shieldscored_Cue.shieldscored_Cue"))))

(event `self.ReceiveBeginPlay`
  (bind _shield (`self.Shield`))
  (bind _returnvalue (`PrimitiveComponent.CreateDynamicMaterialInstance` _shield 0 (`PrimitiveComponent.GetMaterial` _shield 0)))
  (`KismetSystemLibrary.Delay` 120.0)
  (set `self.BossSpawned?` true))

(event `self.ReceiveTick`
  (params (DeltaSeconds :type "Float (single-precision)"))
  (bind _returnvalue (`self.GetInputAxisValue`))
  (bind _opacity (`self.Opacity`))
  (if (!= (`self.BossSpawned?`) true)
    (`self.AddMovementInput` (0.0 -1.0 0.0) (+ 0.37 _returnvalue))
    (else
      (`self.AddMovementInput` (0.0 -1.0 0.0) _returnvalue)))
  ;[1 1 1] Shield Systems on Tick
  (`MaterialInstanceDynamic.SetScalarParameterValue` (stale `self.ReceiveBeginPlay` _returnvalue) "Opacity" (`self.Opacity`))
  (if (`self.IsShieldDown`)
    (`|ExecutionSequence`
      (:`then_0`
        (set `self.Opacity` (- (`self.Opacity`) 0.1)))
      (:`then_1`
        (`/Engine/EditorBlueprintResources/StandardMacros.DoOnce` false :!label _label
          (:`Completed`
            (`GameplayStatics.PlaySoundAtLocation` "/Game/noise/barhit_Cue.barhit_Cue" (`self.K2_GetActorLocation`))
            (set `self.Opacity` 1.0)))))
    (elif (`self.ShieldGot`)
      (if (< _opacity 0.05)
        (set `self.ShieldGot` false)
        (`ActorComponent.SetActive` (`self.Charging`) false false)
        (goto _label :!via `Reset`)
        (else
          (set `self.Opacity` (- _opacity 0.02))))
      (else
        (set `self.Opacity` 0.05)))))

(event `InputAxis|MoveUp`
  (params (AxisValue :type "Float (single-precision)"))
  (`self.AddMovementInput` (0.0 0.0 -1.0) AxisValue))

(event `Key|I`
  (params (Key :type "Key Structure" :default "AnyKey"))
  ;[1 1 1] DEBUG
  (:`Pressed`
    (`/Engine/EditorBlueprintResources/StandardMacros.FlipFlop`
      (:`A`
        (set `self.DebugMode` true)
        (`KismetSystemLibrary.PrintString` "DEBUG" true true (struct :`R` 1.0 :`A` 1.0)))
      (:`B`
        (set `self.DebugMode` false)
        (`KismetSystemLibrary.PrintString` "Normal game" true true (struct :`G` 1.0 :`A` 1.0))))))

(event `Key|L`
  (params (Key :type "Key Structure" :default "AnyKey"))
  ;[1 1 1] DEBUG
  (:`Pressed`
    (if (`self.DebugMode`)
      (if (`self.HaveTBeam`)
        (set `self.DebugMode` false)
        (`self.Dead`)
        (else
          (`self.TBeamGet`))))))

(event `Dead`
  ;[0 0 0] Death
  (if (`self.DebugMode`)
    (`GameplayStatics.PlaySoundAtLocation` "/Game/noise/barhit_Cue.barhit_Cue" (`self.K2_GetActorLocation`))
    (else
      (set `self.IsDead` true)
      (`GameplayStatics.SpawnEmitterAtLocation` "/Game/PARTICLES/A_Boom.A_Boom" (`self.K2_GetActorLocation`))
      (`GameplayStatics.PlaySound2D` "/Game/noise/shipdead_Cue.shipdead_Cue")
      (`MovementComponent.StopMovementImmediately` (`self.CharacterMovement`))
      (`|SpawnActorFromClass` "/Game/Blueprints/coolship_Death.coolship_Death_C" (`self.GetTransform`) "Undefined" "OverrideRootScale")
      (bind _asside_scroller_game_mode (cast `/Game/Blueprints/SideScrollerGameMode` (`GameplayStatics.GetGameMode`)))
      (`/Game/Blueprints/SideScrollerGameMode.Dead` _asside_scroller_game_mode)
      (`self.K2_DestroyActor`))))

(event `Shooting`
  ;[1 1 1] Regular Shooting
  (if (`self.IsFiring`)
    (if (not (`self.TBeamIsCharging`))
      (bind _outactors (`GameplayStatics.GetAllActorsOfClass` "/Game/Blueprints/ShotPlain.ShotPlain_C" :!label _label_2))
      (if (not (> (`KismetArrayLibrary.Array_Length` _outactors) 3))
        (`GameplayStatics.PlaySoundAtLocation` "/Game/noise/shot_Cue.shot_Cue" (`self.K2_GetActorLocation`))
        (`|SpawnActorFromClass` "/Game/Blueprints/ShotPlain.ShotPlain_C" (`SceneComponent.K2_GetComponentToWorld` (`self.Shotspawn`)) "Undefined" "OverrideRootScale"))
      (`KismetSystemLibrary.Delay` 0.1)
      (`self.Shooting`))))

(event `InputAction|Fire`
  (params (Key :type "Key Structure" :default "AnyKey"))
  ;[1 1 1] Regular Shooting
  (:`Pressed`
    (if (not (`self.TBeamIsCharging`))
      (set `self.IsFiring` true)
      (goto _label_2)))
  (:`Released`
    (set `self.IsFiring` false)))

(event `TBeamGet`
  ;[1 1 0] Tension Beam
  ;;[1 1 1] TBeam Collected
  (if (`self.DebugMode`)
    (`GameplayStatics.PlaySound2D` "/Game/noise/TensionBeamAquired_Cue.TensionBeamAquired_Cue" :!label _label_3)
    (set `self.HaveTBeam` true)
    (elif (`self.HaveTBeam`)
      (set `self.Score` (+ (`self.Score`) 10))
      (`GameplayStatics.PlaySound2D` "/Game/noise/shieldscored_Cue.shieldscored_Cue")
      (else
        (goto _label_3)))))

(event `Key|LeftShift`
  (params (Key :type "Key Structure" :default "AnyKey"))
  ;[1 1 0] Tension Beam
  ;;[1 1 1] TBeam Trigger
  (:`Pressed`
    (if (`self.HaveTBeam`)
      (if (not (`self.TBeamIsCharging`))
        (`self.TBeamIsAboutToFire`)))))

(event `TBeamIsAboutToFire`
  ;[1 1 0] Tension Beam
  ;;[1 1 1] TBbeam Active
  (set `self.TBeamIsCharging` true)
  (`ActorComponent.SetActive` (`self.Charging`) true false)
  (`GameplayStatics.PlaySound2D` "/Game/noise/TensionBeam_Cue.TensionBeam_Cue")
  (`KismetSystemLibrary.Delay` 3.2)
  (`ActorComponent.SetActive` (`self.TensionBeam_P`) true false)
  (`ActorComponent.SetActive` (`self.TensionBeam_FiringPoint`) true false)
  (`self.TBeamIsFiring`)
  (`GameplayStatics.PlaySound2D` "/Game/noise/TensionBeamFire_Cue.TensionBeamFire_Cue")
  (if (`self.HaveTBeam`) :!label _label_4
    (`|SpawnActorFromClass` "/Game/Blueprints/TensionBeam.TensionBeam_C" (`SceneComponent.K2_GetComponentToWorld` (`self.Shotspawn`)) "Undefined" "OverrideRootScale")
    (`KismetSystemLibrary.Delay` 0.1)
    (goto _label_4)))

(event `TBeamIsFiring`
  ;[1 1 0] Tension Beam
  ;;[1 1 1] TBeam Trigger event, Duration, and deactivator
  (set `self.TBeamIsDischarging` true)
  (`KismetSystemLibrary.Delay` 7.7)
  (set `self.TBeamIsDischarging` false)
  (`ActorComponent.SetActive` (`self.TensionBeam_FiringPoint`) false false)
  (`GameplayStatics.PlaySound2D` "/Game/noise/TensionBeamPostFire_Cue.TensionBeamPostFire_Cue")
  (set `self.HaveTBeam` false)
  (set `self.TBeamIsCharging` false)
  (`ActorComponent.SetActive` (`self.Charging`) false false)
  (`ActorComponent.SetActive` (`self.TensionBeam_P`) false false)
  (`ActorComponent.SetActive` (`self.Heatvent`) true false)
  (`KismetSystemLibrary.Delay` 3.0)
  (`ActorComponent.SetActive` (`self.Heatvent`) false false))

(fn `AddToScore`
  (set `self.Score` (+ (`self.Score`) 1)))

(fn `UserConstructionScript`)