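; BaddieBoss is a boss enemy that flies a scripted attack pattern and harms the player's ShootingCharacter on contact.
; BeginPlay endlessly loops timed ProjectileMovement velocity changes to weave and lunge.
; Sphere overlap drops the player's shield, or kills an unshielded player and notifies SideScrollerGameMode.
; Tick destroys the boss at zero Health, and Destroyed flags IsBossDead on the player and spawns an enlarged emitter; stay-on-screen logic is unconnected.
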(event `self.ReceiveTick`
  (params (DeltaSeconds :type "Float (single-precision)"))
  (if (<= (`self.Health`) 0)
    (`self.K2_DestroyActor`)))

(event `self.ReceiveBeginPlay`
  (set `MovementComponent.Velocity` (0.0 250.0 0.0) (`self.ProjectileMovement`) :!label _label)
  (`KismetSystemLibrary.Delay` 4.0)
  (set `MovementComponent.Velocity` (-250.0 0.0 -100.0) (`self.ProjectileMovement`))
  (`KismetSystemLibrary.Delay` 0.5)
  (set `MovementComponent.Velocity` (250.0 0.0 -100.0) (`self.ProjectileMovement`))
  (`KismetSystemLibrary.Delay` 0.5)
  (set `MovementComponent.Velocity` (0.0 1700.0 0.0) (`self.ProjectileMovement`))
  (`KismetSystemLibrary.Delay` 0.2)
  (set `MovementComponent.Velocity` (0.0 -1600.0 100.0) (`self.ProjectileMovement`))
  (`KismetSystemLibrary.Delay` 0.85)
  (goto _label))

(event `self.Sphere.OnComponentBeginOverlap`
  (params (OtherActor :type "Actor Object Reference") (OtherComp :type "PrimitiveComponent Object Reference") (OtherBodyIndex :type Integer) (bFromSweep :type Boolean) (SweepResult :type "HitResult Structure (by ref)"))
  (bind _asshooting_character (cast `/Game/Blueprints/ShootingCharacter` OtherActor))
  (if (`/Game/Blueprints/ShootingCharacter.IsShieldDown` _asshooting_character)
    (if (not (`/Game/Blueprints/ShootingCharacter.IsDead` _asshooting_character))
      (`/Game/Blueprints/ShootingCharacter.Dead` _asshooting_character)
      (bind _asside_scroller_game_mode (cast `/Game/Blueprints/SideScrollerGameMode` (`GameplayStatics.GetGameMode`)))
      (`/Game/Blueprints/SideScrollerGameMode.Dead` _asside_scroller_game_mode))
    (else
      (set `/Game/Blueprints/ShootingCharacter.IsShieldDown` true _asshooting_character))))

(event `self.ReceiveDestroyed`
  (bind _asshooting_character (cast `/Game/Blueprints/ShootingCharacter` (`GameplayStatics.GetPlayerPawn` 0)))
  (set `/Game/Blueprints/ShootingCharacter.isBossDead` true _asshooting_character)
  (bind _returnvalue (`GameplayStatics.SpawnEmitterAtLocation` null (`self.K2_GetActorLocation`)))
  (`SceneComponent.SetRelativeScale3D` _returnvalue (5.0 5.0 5.0)))

(fn `UserConstructionScript`)