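; Enemy spawner actor that keeps releasing randomly chosen baddies at its arrow's transform for the first two minutes of play.
; SpawnBaddie re-calls itself after a short random delay until a BeginPlay timer sets StopSpawning.
; Tick holds the spawner at a fixed Y offset from the living ShootingCharacter.
; ListofBaddies fills the class list with two types but is not called here, and the random index range allows a third slot.
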(event `SpawnBaddie`
  ;[1 1 1] Baddie spawning
  (`KismetSystemLibrary.Delay` (`KismetMathLibrary.RandomFloatInRange` 0.1 2.0) :!label _label)
  (if (not (`self.StopSpawning`))
    (`|SpawnActorFromClass` (`KismetArrayLibrary.Array_Get` (`self.BaddieList`) (`KismetMathLibrary.RandomIntegerInRange` 0 2)) (`SceneComponent.K2_GetComponentToWorld` (`self.Arrow`)) "Undefined" "OverrideRootScale")
    (`self.SpawnBaddie`)))

(event `self.ReceiveBeginPlay`
  ;[1 1 1] Baddie spawning
  (`|ExecutionSequence`
    (:`then_0`
      (goto _label))
    (:`then_1`
      (`KismetSystemLibrary.Delay` 120.0)
      (set `self.StopSpawning` true))))

(event `self.ReceiveTick`
  (params (DeltaSeconds :type "Float (single-precision)"))
  (bind _returnvalue (`GameplayStatics.GetPlayerCharacter` 0))
  ;[1 1 1] Stay in the vacinity of the player
  (bind _asshooting_character (cast `/Game/Blueprints/ShootingCharacter` _returnvalue))
  (if (not (`/Game/Blueprints/ShootingCharacter.IsDead` _asshooting_character))
    (`self.K2_SetActorLocation` (`KismetMathLibrary.MakeVector` (.x (`self.K2_GetActorLocation`)) (+ (.y (`self.K2_GetActorLocation` _returnvalue)) -4500.0) (.z (`self.K2_GetActorLocation`))))))

(fn `ListofBaddies`
  (set `self.BaddieList` (`|MakeArray` "/Game/Blueprints/Baddie.Baddie_C" "/Game/Blueprints/BaddieBob.BaddieBob_C" :!type "Actor Class Reference")))

(fn `UserConstructionScript`)